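; BP_VRTarget is an archery target for a VR game that slides back and forth and is destroyed after repeated projectile hits.
; Each tick, a sine of time since creation offsets the collision box along X from its starting position.
; A Projectile overlapping the box is destroyed, switches the target to its hit material and increments the hit count.
; At two hits, it notifies VRGameMode through EventTargetDestroyed and destroys itself.
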(event OnComponentBeginOverlap(BoxCollision)
  (params (OverlappedComponent :type Primitive%20Component%20Object%20Reference) (OtherActor :type Actor%20Object%20Reference) (OtherComp :type Primitive%20Component%20Object%20Reference) (OtherBodyIndex :type Integer) (bFromSweep :type Boolean) (SweepResult :type Hit%20Result%20Structure%20%28by%20ref%29))
  (bind _asprojectile (Utilities|Casting|CastToProjectile OtherActor))
  (Actor|DestroyActor _asprojectile)
  (Rendering|Material|SetMaterial (Variables|Default|GetArcheryTargetStaticMesh) 0 "/Game/MyBlueprints/VRTarget/VRTargetHitMaterial.VRTargetHitMaterial")
  (bind _result (Math|Integer|IncrementInt (Variables|Default|GetHitCount))
    (:%20%20
      (Math|Integer|CompareInt _result 2
        (:==
          (bind _asvrgame_mode (Utilities|Casting|CastToVRGameMode (Game|GetGameMode)))
          (Default|EventTargetDestroyed _asvrgame_mode)
          (Actor|DestroyActor))))))

(event EventBeginPlay
  (Variables|Default|SetBaseLocation (.X (Math|Vector|BreakVector (.Location (Math|Transform|BreakTransform (Transformation|GetRelativeTransform (Variables|Default|GetBoxCollision))))))))

(event EventTick
  (params (DeltaSeconds :type Float%20%28single-precision%29))
  (Transformation|SetRelativeLocation (Variables|Default|GetBoxCollision) (Math|Vector|MakeVector (+ (Variables|Default|GetBaseLocation) (* (Math|Trig|Sin(Degrees) (* (Actor|GetGameTimeSinceCreation) (Variables|Default|GetSpeed))) (Variables|Default|GetBobbingDistance))) 0.0 0.0) false false))

(fn ConstructionScript)